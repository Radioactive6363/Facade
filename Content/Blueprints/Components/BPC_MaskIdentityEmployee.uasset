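; BPC_MaskIdentityEmployee is an employee mask identity component that runs an interaction action and can change the interactor's rank.
; SetData calls the parent version, then constructs the ActionOnInteraction object from the class in the mask data.
; ExecuteAction binds to that action's success dispatcher and initializes it with interactor and owner.
; MaskSteal sends a rank change through BPI_PlayerGameplay if the interactor implements it.
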(event Custom|MaskSteal
  (params (Interactor :type Actor%20Object%20Reference))
  (if (Utilities|DoesObjectImplementInterface Interactor "/Game/Blueprints/Interfaces/BPI_PlayerGameplay.BPI_PlayerGameplay_C")
    (Class|BPIPlayerGameplay|ChangePlayerRank(Message) Interactor (Variables|Default|GetRank))))

(event Custom|ExecuteAction
  (params (Interactor :type Actor%20Object%20Reference) (Owner :type Actor%20Object%20Reference))
  (bind _actiononinteraction (Variables|Default|GetActionOnInteraction))
  (EventDispatchers|BindEventtoOnSuccededAction _actiononinteraction (EventDispatchers|CreateEvent :!event Custom|MaskSteal))
  (Default|OnInitialize _actiononinteraction Interactor Owner))

(fn SetData
  (params (MaskData :type ST%20Mask%20Infrastructure%20Structure))
  (|CallParentFunction MaskData)
  (bind _returnvalue (Game|ConstructObjectfromClass (.ActionOnInteraction (Utilities|Struct|BreakST_MaskInfrastructure MaskData))))
  (Variables|Default|SetActionOnInteraction _returnvalue))