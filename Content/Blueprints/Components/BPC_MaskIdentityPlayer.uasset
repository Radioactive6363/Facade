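; Player mask identity component that colors its owner's meshes according to mask Rank.
; On BeginPlay it gets the owner's base meshes and puts one shared dynamic instance of MI_MaskRank on every material slot.
; ChangeMask fetches rank data from the GameInstance, sets the material's BaseColor, and writes a color-derived custom depth stencil value to each mesh.
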(event EventBeginPlay
  (Initialize|ObtainOwnerMeshes)
  (bind _returnvalue (Rendering|Material|CreateDynamicMaterialInstance "/Game/Material/MI_MaskRank.MI_MaskRank" "None" "None" :!class /Script/Engine.KismetMaterialLibrary))
  (bind _output_get (Variables|Default|SetMaskMaterial _returnvalue))
  (for _array_element (Variables|Default|GetOwnerMeshes)
    (Initialize|AssignDynamicMaterialtoMesh _array_element _output_get))
  (MainFunctions|ChangeMask (Variables|Default|GetRank)))

(fn GetData
  (params (Rank :type EM_MaskRanks%20Enum :default "NewEnumerator0"))
  (bind _maskdata (Class|BPIGameManagerComms|GetMaskData(Message) (Game|GetGameInstance) Rank))
  (return _maskdata))

(fn SetData
  (params (MaskData :type ST%20Mask%20Infrastructure%20Structure))
  (MainFunctions|ChangeColor (.RankTexture (Utilities|Struct|BreakST_MaskInfrastructure MaskData))))

(fn ChangeMask
  (params (Rank :type EM_MaskRanks%20Enum :default "NewEnumerator0"))
  (bind _output_get (Variables|Default|SetRank Rank))
  (bind _maskdata (MainFunctions|GetData _output_get))
  (MainFunctions|SetData _maskdata))

(fn ChangeColor
  (params (LinearColor :type Linear%20Color%20Structure))
  (Rendering|Material|SetVectorParameterValue (Variables|Default|GetMaskMaterial) "BaseColor" LinearColor :!class /Script/Engine.MaterialInstanceDynamic)
  (for _array_element (Variables|Default|GetOwnerMeshes)
    (Rendering|SetCustomDepthStencilValue _array_element (CallFunction|ColortoStencilValue LinearColor)))
  (return))

(fn AssignDynamicMaterialtoMesh
  (params (Mesh :type Mesh%20Component%20Object%20Reference) (MaskMaterial :type Material%20Instance%20Dynamic%20Object%20Reference))
  (for _index (range 0 (- (Rendering|Material|GetNumMaterials Mesh) 1))
    (Rendering|Material|SetMaterial Mesh _index MaskMaterial))
  (return))

(fn ObtainOwnerMeshes
  (bind _meshes (Class|BPIGetBaseMeshes|GetBaseMeshes(Message) (Components|GetOwner)))
  (Variables|Default|SetOwnerMeshes _meshes)
  (return))