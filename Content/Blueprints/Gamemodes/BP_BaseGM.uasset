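; Base game mode that handles losing and restarting a level.
; On lose, it swaps all Enhanced Input mappings for a lose mapping context, removes the player's base widget and shows a lose widget.
; Restart reopens the current level by name, and BeginPlay starts background audio through a game instance message.
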(event EventBeginPlay
  (Class|BPIGameManagerComms|Start/StopBackgroundAudio(Message) (Game|GetGameInstance) true))

(event EventCallRestart
  (bind _returnvalue (Game|GetCurrentLevelName true))
  (Game|OpenLevel(byName) (Utilities|String|StringToName _returnvalue)))

(event EventCallLose
  (Utilities|FlowControl|Sequence
    (:then_0
      (CallFunction|RemoveAllMappingsfromPlayer)
      (CallFunction|AddLoseMapping))
    (:then_1
      (CallFunction|RemoveBaseWidget))
    (:then_2
      (bind _returnvalue (UserInterface|CreateWidget "/Game/Blueprints/Widgets/Gameplay/WB_LoseWidget.WB_LoseWidget_C" (Game|GetPlayerController 0)))
      (bind _output_get (Variables|Default|SetLoseWidget _returnvalue))
      (UserInterface|Viewport|AddtoViewport _output_get 0))))

(fn ConstructionScript)

(fn RemoveBaseWidget
  (bind _basewidget (Class|BPIPlayerController|GetBaseWidget(Message) (Game|GetPlayerController 0)))
  (Widget|RemovefromParent _basewidget))

(fn RemoveAllMappingsfromPlayer
  (Class|EnhancedInputSubsystemInterface|ClearAllMappings (PlayerController|LocalPlayerSubsystems|GetEnhancedInputLocalPlayerSubsystem (Game|GetPlayerController 0))))

(fn AddLoseMapping
  (Input|AddMappingContext (PlayerController|LocalPlayerSubsystems|GetEnhancedInputLocalPlayerSubsystem (Game|GetPlayerController 0)) "/Game/Input/IMC_LoseMapping.IMC_LoseMapping" 0 "(bIgnoreAllPressedKeysUntilRelease=True,bForceImmediately=False,bNotifyUserSettings=False)"))