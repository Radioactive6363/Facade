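; GI_DataManager is a game instance that serves mask data and controls global 2D audio.
; On Init it synchronously loads the BP_MaskData library, which GetMaskData searches by Rank, printing an error on failure.
; Audio events play or stop the tension loop, spawned on first use, and fade suspicion audio in or out.
; The suspicion fade-in runs only if that audio is already playing, and its spawn reuses its own variable as the source.
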(event EventInit
  (CallFunction|MaskDataInitialize))

(event EventStart/StopBackgroundAudio
  (params (PlayAudio? :type Boolean))
  (Utilities|IsValid (Variables|Default|GetBackgroundAudio)
    (:Is%20Valid
      _)
    (:Is%20Not%20Valid
      (bind _returnvalue (Audio|SpawnSound2D "/Game/Audio/SW_TensionLoop.SW_TensionLoop" 1.0 1.0 0.0 0))
      (Variables|Default|SetBackgroundAudio _returnvalue)))
  (if PlayAudio?
    (Audio|Components|Audio|Play (Variables|Default|GetBackgroundAudio) 0.0)
    (else
      (Audio|Components|Audio|Stop (Variables|Default|GetBackgroundAudio)))))

(event EventStart/StopSuspicionAudio
  (params (Play? :type Boolean))
  (Utilities|IsValid (Variables|Default|GetSuspicionSounds)
    (:Is%20Valid
      _)
    (:Is%20Not%20Valid
      (bind _returnvalue (Audio|SpawnSound2D "/Game/Audio/SuspicionSounds.SuspicionSounds" 1.0 1.0 0.0 0))
      (Variables|Default|SetSuspicionSounds _returnvalue)))
  (if Play?
    (if (Audio|Components|Audio|IsPlaying (Variables|Default|GetSuspicionSounds))
      (Audio|Components|Audio|FadeIn (Variables|Default|GetSuspicionSounds) 1.0 1.0 0.0 "Linear" :!class /Script/Engine.AudioComponent))
    (else
      (Audio|Components|Audio|FadeOut (Variables|Default|GetSuspicionSounds) 1.0 0.0 "Linear" :!class /Script/Engine.AudioComponent))))

(fn MaskDataInitialize
  (bind _returnvalue (Utilities|LoadAssetBlocking (Variables|Default|GetMaskLibraryDirectory)))
  (bind _asbp_mask_data (Utilities|Casting|CastToBP_MaskData _returnvalue)
    (:then
      (Variables|Default|SetMaskLibrary _asbp_mask_data))
    (:CastFailed
      (Development|PrintString "Failed Loading BP_MaskData"))))

(fn GetMaskData
  (params (Rank :type EM_MaskRanks%20Enum :default "NewEnumerator5"))
  (bind _masklibrary (Variables|Default|GetMaskLibrary))
  (bind (_value _returnvalue) (Utilities|Map|Find (Variables|/Game/Blueprints/Data/BP_MaskData.BP_MaskData_C|GetRank _masklibrary) Rank))
  (if _returnvalue
    (return _value)
    (else
      (Development|PrintString "Failed Loading Mask Data from GI")
      (return ""))))