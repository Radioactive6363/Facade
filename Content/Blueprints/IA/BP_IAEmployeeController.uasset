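; AI controller for an employee NPC that catches the player stealing a message and triggers the game's lose message.
; It runs a behavior tree and checks the player's stealing state on perception updates.
; Detection sets HasLineOfSight, stops movement, and starts timers for turning toward the player and for the delayed loss.
; Any perception update without a sensed, stealing player cancels an active countdown and clears the flag.
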(event OnTargetPerceptionUpdated(AIPerception)
  (params (Actor :type Actor%20Object%20Reference) (Stimulus :type AI%20Stimulus%20Structure))
  (bind _returnvalue (Game|GetPlayerCharacter 0))
  (if (and (== Actor _returnvalue) (.bSuccessfullySensed (Utilities|Struct|BreakAIStimulus Stimulus)))
    (bind _stealing_ (Class|BPIPlayerGameplay|IsPlayerStealing?(Message) _returnvalue))
    (if _stealing_
      (Variables|Default|SetPlayerDetected _returnvalue)
      (if (not (Utilities|Time|IsTimerActivebyHandle (Variables|Default|GetVisibleTimer)))
        (CallFunction|StopIA)
        (bind _returnvalue_2 (Utilities|Time|SetTimerbyEvent (EventDispatchers|CreateEvent :!event Custom|OnWatched) (Variables|Default|GetTimeToSee)))
        (Variables|Default|SetVisibleTimer _returnvalue_2))
      (else
        (if (Utilities|Time|IsTimerActivebyHandle (Variables|Default|GetVisibleTimer)) :!label _label
          (AI|Components|Blackboard|SetValueasBool (AI|GetBlackboard 0) (Utilities|Name|MakeLiteralName "HasLineOfSight") false)
          (Variables|Default|SetPlayerDetected 0)
          (Utilities|Time|ClearandInvalidateTimerbyHandle (Variables|Default|GetWatchPlayerHandler))
          (Utilities|Time|ClearandInvalidateTimerbyHandle (Variables|Default|GetVisibleTimer)))))
    (else
      (goto _label))))

(event Custom|OnWatched
  (Class|BPIGameModeComm|CallLose(Message) (Game|GetGameMode)))

(event Custom|StopIA
  (AI|Components|Blackboard|SetValueasBool (AI|GetBlackboard 0) (Utilities|Name|MakeLiteralName "HasLineOfSight") true)
  (AI|Navigation|StopMovement)
  (bind _returnvalue (Utilities|Time|SetTimerbyEvent (EventDispatchers|CreateEvent :!event Custom|WatchTowardsPlayer) 0.01 true))
  (Variables|Default|SetWatchPlayerHandler _returnvalue))

(event Custom|WatchTowardsPlayer
  (bind _returnvalue (Pawn|GetControlledPawn))
  (bind _playerdetected (Variables|Default|GetPlayerDetected))
  (Utilities|IsValid _playerdetected
    (:Is%20Valid
      (Transformation|SetActorRotation _returnvalue (Math|Rotator|FindLookatRotation (Transformation|GetActorLocation _returnvalue) (Transformation|GetActorLocation _playerdetected))))))

(event EventBeginPlay
  (AI|RunBehaviorTree (Variables|Default|GetBTAsset)))

(fn ConstructionScript)