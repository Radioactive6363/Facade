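; Timed employee character action in which an Interactor hacks or steals, with messages toggled on the Interactor.
; A looping timer adds progress while the owner's AI controller has the Interactor in sight within its forward cone, pausing otherwise.
; When visible, a failed range check, which compares world-position vector lengths rather than true separation, resets the action.
; Reaching the maximum time resets it and fires the success callback.
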(event Custom|OnSucceded
  (CallFunction|ResetAction)
  (Default|CallOnSuccededAction (Variables|Default|GetInteractor)))

(event Custom|OnInitialize
  (params (Interactor :type Actor%20Object%20Reference) (ActionOwner :type Actor%20Object%20Reference))
  (Variables|Default|SetInteractor Interactor)
  (Variables|Default|SetAction%20Owner ActionOwner)
  (Class|BPIPlayerGameplay|Enable/DisableInteracting(Message) (Variables|Default|GetInteractor) false)
  (Class|BPIPlayerGameplay|SetPlayerStealing(Message) (Variables|Default|GetInteractor) true)
  (Utilities|Time|SetTimerbyFunctionName 0 "Hacking" (Variables|Default|GetTimerSpeed) true))

(event Custom|Hacking
  (bind _detected_ (CallFunction|CheckLineOfSight (Variables|Default|GetAction%20Owner) (Variables|Default|GetInteractor)))
  (if _detected_
    (bind _isnear_ (CallFunction|GetDistance))
    (if _isnear_
      (bind _output_get (Variables|Default|SetCurrentHackingProgress (+ (Variables|Default|GetCurrentHackingProgress) (Variables|Default|GetTimerSpeed))))
      (Development|PrintString (Variables|Default|GetAction%20Owner) (Utilities|String|ToString(Float) _output_get))
      (if (>= _output_get (Variables|Default|GetMaxHackingTime))
        (Utilities|FlowControl|DoOnce false
          (:Completed
            (CallFunction|OnSucceded))))
      (else
        (CallFunction|ResetAction)))))

(event Custom|ResetAction
  (bind _interactor (Variables|Default|GetInteractor))
  (Utilities|Time|ClearTimerbyFunctionName 0 "Hacking")
  (Class|BPIPlayerGameplay|Enable/DisableInteracting(Message) _interactor true)
  (Class|BPIPlayerGameplay|SetPlayerStealing(Message) _interactor false)
  (Variables|Default|SetCurrentHackingProgress 0.0)
  (Utilities|FlowControl|DoOnce false) ; enters at Reset
)

(fn GetDistance
  (return (> (Variables|Default|GetMaxDistance) (- (Math|Vector|VectorLength (Transformation|GetActorLocation (Variables|Default|GetAction%20Owner))) (Math|Vector|VectorLength (Transformation|GetActorLocation (Variables|Default|GetInteractor)))))))

(fn CheckLineOfSight
  (params (ControlledActor :type Actor%20Object%20Reference) (Other :type Actor%20Object%20Reference))
  (return (and (Controller|LineOfSightTo (AI|GetAIController ControlledActor) Other "0, 0, 0" false) (> (Math|Vector|DotProduct (Transformation|GetActorForwardVector ControlledActor) (Math|Vector|Normalize (- (Transformation|GetActorLocation Other) (Transformation|GetActorLocation ControlledActor)))) 0.6))))