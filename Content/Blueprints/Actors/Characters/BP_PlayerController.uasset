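; Player controller that sets up base input and the player HUD.
; On BeginPlay it adds the IMC_PlayerBaseInput mapping context to the Enhanced Input subsystem, then creates WB_PlayerHUD and adds it to the viewport.
; It keeps the HUD reference and exposes its OverlayBase through GetWidgetOverlayContainer.
; The Manaos event is an empty stub.
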(event Custom|Manaos)

(event EventBeginPlay
  (Utilities|FlowControl|Sequence
    (:then_0
      (Input|AddMappingContext (PlayerController|LocalPlayerSubsystems|GetEnhancedInputLocalPlayerSubsystem self) "/Game/Input/IMC_PlayerBaseInput.IMC_PlayerBaseInput" 0 "(bIgnoreAllPressedKeysUntilRelease=True,bForceImmediately=False,bNotifyUserSettings=False)"))
    (:then_1
      (bind _returnvalue (UserInterface|CreateWidget "/Game/Blueprints/Widgets/Gameplay/WB_PlayerHUD.WB_PlayerHUD_C" self))
      (bind _output_get (Variables|Default|SetPlayerWidget _returnvalue))
      (UserInterface|Viewport|AddtoViewport _output_get 0))))

(fn ConstructionScript)

(fn GetWidgetOverlayContainer
  (return (Variables|/Game/Blueprints/Widgets/Gameplay/WB_PlayerHUD.WB_PlayerHUD_C|GetOverlayBase (Variables|Default|GetPlayerWidget))))