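; BP_Employee is an interactable employee character whose rank and interaction action come from its BPCMaskIdentityEmployee component.
; It allows interaction only when the instigator implements BPI_PlayerGameplay and its rank is exactly one step below the employee's.
; A completed interaction passes the interactor to the component's ExecuteAction, while the actor supplies a fixed interaction time and a hover prompt showing the rank.
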(event EventDoInteractionResult
  (params (HitResult :type Hit%20Result%20Structure) (Interactor :type Actor%20Object%20Reference))
  (Default|ExecuteAction (Variables|Default|GetBPC_MaskIdentityEmployee) Interactor self))

(fn ConstructionScript
  (|CallParentFunction))

(fn CanbeInteracted
  (params (Instigator :type Actor%20Object%20Reference))
  (if (Utilities|DoesObjectImplementInterface Instigator "/Game/Blueprints/Interfaces/BPI_PlayerGameplay.BPI_PlayerGameplay_C")
    (bind _rank (Class|BPIPlayerGameplay|CheckPlayerRank(Message) Instigator))
    (return (== (+ (Math|Conversions|ToInteger(Byte) _rank) 1) (Math|Conversions|ToInteger(Byte) (Variables|/Game/Blueprints/Components/BPC_MaskIdentityPlayer.BPC_MaskIdentityPlayer_C|GetRank (Variables|Default|GetBPC_MaskIdentityEmployee)))))))

(fn GetTime
  (return 1.0))

(fn IsHoveringActor
  (params (Hit :type Hit%20Result%20Structure) (Interactor :type Actor%20Object%20Reference))
  (return (Utilities|Text|FormatText "Interact with {Rank}" (|GenerictoText (Variables|/Game/Blueprints/Components/BPC_MaskIdentityPlayer.BPC_MaskIdentityPlayer_C|GetRank (Variables|Default|GetBPC_MaskIdentityEmployee))))))