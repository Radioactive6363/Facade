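; BP_CoinProjectile is a coin actor that flies and bounces with sound, and reports itself as non-interactable.
; Initialize sets a stencil value from the coin color and makes the mesh the projectile movement's updated component.
; Hard bounces play a random positional coin sound, while slow impacts switch the mesh to physics simulation and stop rotation following velocity.
; ActivateDeactivate toggles visibility and component ticking, playing a spawn sound on activation.
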(event OnProjectileStop(ProjectileMovement)
  (params (ImpactResult :type Hit%20Result%20Structure%20%28by%20ref%29)))

(event OnProjectileBounce(ProjectileMovement)
  (params (ImpactResult :type Hit%20Result%20Structure%20%28by%20ref%29) (ImpactVelocity :type Vector%20%28by%20ref%29 :default "0, 0, 0"))
  (if (> (Math|Vector|VectorLength ImpactVelocity) 1.5e+02)
    (Audio|PlaySoundatLocation (.OutItem (Utilities|Array|Random (Variables|Default|GetCoinSounds))) (.Location (Collision|BreakHitResult ImpactResult)) "0, 0, 0" 1.0 1.0 0.0 "/Game/Audio/SA_Coin.SA_Coin" 0 self 0)
    (else
      (Physics|SetSimulatePhysics (Variables|Default|GetStaticMesh) true)
      (Variables|/Script/Engine.ProjectileMovementComponent|SetbRotationFollowsVelocity (Variables|Default|GetProjectileMovement) false))))

(event EventBeginPlay
  (CallFunction|Initialize))

(fn ConstructionScript
  (|CallParentFunction))

(fn Activate/Deactivate
  (params (Activate? :type Boolean))
  (Rendering|SetActorHiddenInGame (not Activate?))
  (Components|Tick|SetComponentTickEnabled (Variables|Default|GetStaticMesh) Activate?)
  (Components|Tick|SetComponentTickEnabled (Variables|Default|GetProjectileMovement) Activate?)
  (bind _output_get (Variables|Default|SetIsActive? Activate?))
  (if _output_get
    (Audio|PlaySound2D (Variables|Default|GetCoinSpawnSound) 1.0 1.0 0.0 0 0)))

(fn Initialize
  (Rendering|SetCustomDepthStencilValue (Variables|Default|GetStaticMesh) (CallFunction|ColortoStencilValue (Variables|Default|GetCoinColor)))
  (Components|Movement|SetUpdatedComponent (Variables|Default|GetProjectileMovement) (Variables|Default|GetStaticMesh))
  (return))

(fn CanbeInteracted
  (params (Instigator :type Actor%20Object%20Reference))
  (return false))

(fn GetTime
  (return 0.0))

(fn IsHoveringActor
  (params (Hit :type Hit%20Result%20Structure) (Interactor :type Actor%20Object%20Reference))
  (return ""))