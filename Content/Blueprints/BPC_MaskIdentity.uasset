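; BPC_MaskIdentity is an actor component that recolors its owner's meshes to show a mask rank.
; On BeginPlay it fetches the owner's meshes through a message call and applies one shared dynamic instance of MI_MaskRank to every material slot.
; It then queries the GameInstance for the DesiredRank's data and writes the returned RankTexture value, used as a color, to the BaseColor parameter.
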(event EventBeginPlay
  (Initialize|ObtainOwnerMeshes)
  (bind _returnvalue (Rendering|Material|CreateDynamicMaterialInstance "/Game/Material/MI_MaskRank.MI_MaskRank" "None" "None" :!class /Script/Engine.KismetMaterialLibrary))
  (bind _output_get (Variables|Default|SetMaskMaterial _returnvalue))
  (for _array_element (Variables|Default|GetOwnerMeshes)
    (Initialize|AssignDynamicMaterialtoMesh _array_element _output_get))
  (Development|PrintString "Done Replacing Materials")
  (MainFunctions|GetData (Variables|Default|GetDesiredRank)))

(fn GetData
  (params (Rank :type EM_MaskRanks%20Enum :default "NewEnumerator0"))
  (bind _maskdata (Class|BPIGameManagerComms|GetMaskData(Message) (Game|GetGameInstance) Rank))
  (MainFunctions|ChangeMaterial (.RankTexture (Utilities|Struct|BreakST_MaskInfrastructure _maskdata))))

(fn ChangeMaterial
  (params (LinearColor :type Linear%20Color%20Structure))
  (Rendering|Material|SetVectorParameterValue (Variables|Default|GetMaskMaterial) "BaseColor" LinearColor :!class /Script/Engine.MaterialInstanceDynamic))

(fn AssignDynamicMaterialtoMesh
  (params (Mesh :type Mesh%20Component%20Object%20Reference) (MaskMaterial :type Material%20Instance%20Dynamic%20Object%20Reference))
  (for _index (range 0 (- (Rendering|Material|GetNumMaterials Mesh) 1))
    (Rendering|Material|SetMaterial Mesh _index MaskMaterial))
  (Development|PrintString "Suceeded changin materials")
  (return))

(fn ObtainOwnerMeshes
  (bind _meshes (Class|BPIGetBaseMeshes|GetBaseMeshes(Message) (Components|GetOwner)))
  (Variables|Default|SetOwnerMeshes _meshes)
  (return))