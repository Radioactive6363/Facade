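; GI_DataManager is a Game Instance Blueprint that gives the game access to mask data.
; On Init it synchronously loads the asset referenced by MaskLibraryDirectory, casts it to BP_MaskData and caches it as MaskLibrary.
; GetMaskData looks up a given rank in that library's Rank map and returns the matching entry.
; A failed cast or missing rank prints an error string.
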(event EventInit
  (bind _returnvalue (Utilities|LoadAssetBlocking (Variables|Default|GetMaskLibraryDirectory)))
  (bind _asbp_mask_data (Utilities|Casting|CastToBP_MaskData _returnvalue)
    (:then
      (Variables|Default|SetMaskLibrary _asbp_mask_data))
    (:CastFailed
      (Development|PrintString "Failed Loading BP_MaskData"))))

(fn GetMaskData
  (params (Rank :type EM_MaskRanks%20Enum :default "NewEnumerator0"))
  (bind _masklibrary (Variables|Default|GetMaskLibrary))
  (bind (_value _returnvalue) (Utilities|Map|Find (Variables|/Game/Blueprints/Data/BP_MaskData.BP_MaskData_C|GetRank _masklibrary) Rank))
  (if _returnvalue
    (return _value)
    (else
      (Development|PrintString "Failed Loading Mask Data from GI")
      (return ""))))